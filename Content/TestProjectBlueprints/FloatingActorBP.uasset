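; FloatingActorBP is an actor that displays its world height through a HeightMeter widget on its UIPart component.
; Both the construction script and BeginPlay create a HeightMeter, store it and assign it to UIPart.
; Each Tick copies the world Z of DefaultSceneRoot into the widget's Height property.
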(event EventBeginPlay
  (bind _returnvalue (Game|ConstructObjectfromClass "/Game/TestProjectBlueprints/HeightMeter.HeightMeter_C" (Variables|Default|GetUIPart)))
  (bind _output_get (Variables|Default|SetHeightMeter _returnvalue))
  (UserInterface|SetWidget (Variables|Default|GetUIPart) _output_get))

(event Collision|EventActorBeginOverlap
  (params (OtherActor :type Actor%20Object%20Reference)))

(event EventTick
  (params (DeltaSeconds :type Float%20%28single-precision%29))
  (Variables|/Game/TestProjectBlueprints/HeightMeter.HeightMeter_C|SetHeight (Variables|Default|GetHeightMeter) (.z (Transformation|GetWorldLocation (Variables|Default|GetDefaultSceneRoot)))))

(fn ConstructionScript
  (bind _returnvalue (Game|ConstructObjectfromClass "/Game/TestProjectBlueprints/HeightMeter.HeightMeter_C" (Variables|Default|GetUIPart)))
  (bind _output_get (Variables|Default|SetHeightMeter _returnvalue))
  (UserInterface|SetWidget (Variables|Default|GetUIPart) _output_get))